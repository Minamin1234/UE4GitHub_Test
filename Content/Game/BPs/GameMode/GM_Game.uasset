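; Game mode that manages which UI widget is on screen, creating an initial widget on BeginPlay.
; SelectWidget clears all widgets, creates the one for the chosen screen, then adds it to the viewport and shows the mouse cursor.
; The None and Game cases return early, skipping that shared step; Game hides the cursor instead.
; ShowWidget creates and displays any valid widget class without clearing existing ones.
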(event `self.ReceiveBeginPlay`
  (`self.Initialize`))

(fn `Initialize`
  (`WidgetLayoutLibrary.RemoveAllWidgets`)
  (bind _returnvalue (`|CreateWidget` (`self.Initial Widget`) (`GameplayStatics.GetPlayerController` 0)))
  (`UserWidget.AddToViewport` _returnvalue 0))

(fn `SelectWidget`
  (params (Select :type "/Game/Game/BPs/Widgets/E_SelectWidget Enum" :default "NewEnumerator5"))
  (returns (CreatedWidget :type "UserWidget Object Reference") (`Selected Widget` :type "/Game/Game/BPs/Widgets/E_SelectWidget Enum"))
  (locals (CurrentWidget :type "UserWidget Object Reference"))
  (bind _returnvalue (`GameplayStatics.GetPlayerController` 0))
  (`WidgetLayoutLibrary.RemoveAllWidgets`)
  (`|ExecutionSequence`
    (:`then_0`
      (switch `/Game/Game/BPs/Widgets/E_SelectWidget` Select
        (:`NewEnumerator5`
          (`WidgetLayoutLibrary.RemoveAllWidgets`)
          (return null "NewEnumerator5"))
        (:`NewEnumerator0`
          (bind _returnvalue_2 (`|CreateWidget` (`self.Title Widget`) _returnvalue))
          (set `local.CurrentWidget` _returnvalue_2))
        (:`NewEnumerator1`
          (bind _returnvalue_3 (`|CreateWidget` (`self.Menu Widget`) _returnvalue))
          (set `local.CurrentWidget` _returnvalue_3))
        (:`NewEnumerator2`
          (bind _returnvalue_4 (`|CreateWidget` (`self.Inventory Widget`) _returnvalue))
          (set `local.CurrentWidget` _returnvalue_4))
        (:`NewEnumerator3`
          (bind _returnvalue_5 (`|CreateWidget` (`self.Settings Widget`) _returnvalue))
          (set `local.CurrentWidget` _returnvalue_5))
        (:`NewEnumerator4`
          (bind _returnvalue_6 (`|CreateWidget` (`self.Player Widget`) _returnvalue))
          (bind _output_get (set `local.CurrentWidget` _returnvalue_6))
          (set `PlayerController.bShowMouseCursor` false (`GameplayStatics.GetPlayerController` 0))
          (return _output_get (`local.Select`)))))
    (:`then_1`
      (`UserWidget.AddToViewport` (`local.CurrentWidget`) 0)
      (set `PlayerController.bShowMouseCursor` true (`GameplayStatics.GetPlayerController` 0)))
    (:`then_2`
      (return (`local.CurrentWidget`) (`local.Select`)))))

(fn `ShowWidget`
  (params (Class :type "UserWidget Class Reference"))
  (returns (`Created Widget` :type "UserWidget Object Reference") (ReturnValue :type Boolean))
  (locals (CurrentWidget :type "UserWidget Object Reference"))
  (bind _returnvalue (`KismetSystemLibrary.IsValidClass` Class))
  (if _returnvalue
    (bind _returnvalue_2 (`|CreateWidget` Class (`GameplayStatics.GetPlayerController` 0)))
    (bind _output_get (set `local.CurrentWidget` _returnvalue_2))
    (`UserWidget.AddToViewport` _output_get 0)
    (return (`local.CurrentWidget`) _returnvalue)))

(fn `UserConstructionScript`)