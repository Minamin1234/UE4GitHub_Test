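; Player character Blueprint handling movement, jump, camera look, sprint, widget toggling and save slot access.
; Movement follows control yaw to stay ground-parallel, and sprint multiplies MaxWalkSpeed while held, dividing it back on release.
; Q and I each flip-flop between two widgets through GM_Game.SelectWidget, caching the result.
; BeginPlay optionally loads the save object without applying it; Save, uncalled here, writes a self reference to an SBP_SaveGame slot.
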(event `self.ReceiveBeginPlay`
  (`|ExecutionSequence`
    (:`then_0`
      (`self.Load`))))

(event `InputAxis|MoveForward`
  (params (AxisValue :type "Float (single-precision)"))
  ;[1 1 1] 前方向への移動
  (`self.AddMovementInput` (`KismetMathLibrary.GetForwardVector` (`KismetMathLibrary.MakeRotator` 0.0 0.0 (.yaw (`self.GetControlRotation`)))) AxisValue))

(event `InputAxis|MoveRight`
  (params (AxisValue :type "Float (single-precision)"))
  ;[1 1 1] 横方向への移動
  (`self.AddMovementInput` (`KismetMathLibrary.GetRightVector` (`KismetMathLibrary.MakeRotator` 0.0 0.0 (.yaw (`self.GetControlRotation`)))) AxisValue))

(event `InputAction|Jump`
  (params (Key :type "Key Structure"))
  ;[1 1 1] 単なるジャンプ処理
  (:`Pressed`
    (`self.Jump`)))

(event `InputAxis|LookUp`
  (params (AxisValue :type "Float (single-precision)"))
  (`self.AddControllerPitchInput` AxisValue) ; カメラの回転
)

(event `InputAxis|Turn`
  (params (AxisValue :type "Float (single-precision)"))
  (`self.AddControllerYawInput` AxisValue) ; カメラの回転
)

(event `self.ReceiveTick`
  (params (DeltaSeconds :type "Float (single-precision)")))

(event `InputAction|Sprint`
  (params (Key :type "Key Structure"))
  (bind _charactermovement (`self.CharacterMovement`))
  ;[1 1 1] ダッシュ
  (:`Pressed`
    ;;[1 1 1] 通常の歩行速度に指定された倍数をかける。
    (set `self.IsSprint` true) ; 走っている
    (set `CharacterMovementComponent.MaxWalkSpeed` (* (`CharacterMovementComponent.MaxWalkSpeed` _charactermovement) (`self.SprintSpeedScale`)) _charactermovement))
  (:`Released`
    (set `self.IsSprint` false) ; 歩いている
    (set `CharacterMovementComponent.MaxWalkSpeed` (/ (`CharacterMovementComponent.MaxWalkSpeed` _charactermovement) (`self.SprintSpeedScale`)) _charactermovement)))

(event `InputAction|Q_Clicked`
  (params (Key :type "Key Structure"))
  (:`Pressed`
    (`/Engine/EditorBlueprintResources/StandardMacros.DoOnce` false :!label _label
      (:`Completed`
        (`/Engine/EditorBlueprintResources/StandardMacros.FlipFlop`
          (:`A`
            (bind _asgm_game (cast `/Game/Game/BPs/GameMode/GM_Game` (`GameplayStatics.GetGameMode`)))
            (bind (_createdwidget _selected_widget) (`/Game/Game/BPs/GameMode/GM_Game.SelectWidget` _asgm_game "NewEnumerator1"))
            (set `self.CurrentWidget` _createdwidget)
            (set `self.Showing Widget` _selected_widget))
          (:`B`
            (bind _asgm_game_2 (cast `/Game/Game/BPs/GameMode/GM_Game` (`GameplayStatics.GetGameMode`)))
            (bind (_createdwidget_2 _selected_widget_2) (`/Game/Game/BPs/GameMode/GM_Game.SelectWidget` _asgm_game_2 "NewEnumerator5"))
            (set `self.CurrentWidget` _createdwidget_2)
            (set `self.Showing Widget` _selected_widget_2))))))
  (:`Released`
    (goto _label :!via `Reset`)))

(event `InputAction|I_Clicked`
  (params (Key :type "Key Structure"))
  (:`Pressed`
    (`/Engine/EditorBlueprintResources/StandardMacros.DoOnce` false :!label _label
      (:`Completed`
        (bind _asgm_game (cast `/Game/Game/BPs/GameMode/GM_Game` (`GameplayStatics.GetGameMode`)))
        (`/Engine/EditorBlueprintResources/StandardMacros.FlipFlop`
          (:`A`
            (bind (_createdwidget _selected_widget) (`/Game/Game/BPs/GameMode/GM_Game.SelectWidget` _asgm_game "NewEnumerator2"))
            (set `self.Showing Widget` _selected_widget)
            (set `self.CurrentWidget` _createdwidget))
          (:`B`
            (bind (_createdwidget_2 _selected_widget_2) (`/Game/Game/BPs/GameMode/GM_Game.SelectWidget` _asgm_game "NewEnumerator4"))
            (set `self.Showing Widget` _selected_widget_2)
            (set `self.CurrentWidget` _createdwidget_2))))))
  (:`Released`
    (goto _label :!via `Reset`)))

(fn `Load`
  (if (`self.IsLoad`)
    (bind _returnvalue (`GameplayStatics.LoadGameFromSlot` (`self.SaveSlot`)))
    (set `self.SaveGameClass` _returnvalue)))

(fn `Save`
  (returns (IsSaved :type Boolean))
  (if (`self.IsSave`)
    (bind _returnvalue (`GameplayStatics.CreateSaveGameObject` "/Game/Game/BPs/Save/SBP_SaveGame.SBP_SaveGame_C"))
    (bind _output_get (set `self.SaveGameClass` _returnvalue))
    (bind _assbp_save_game (cast `/Game/Game/BPs/Save/SBP_SaveGame` _output_get))
    (set `/Game/Game/BPs/Save/SBP_SaveGame.Player` self _assbp_save_game)
    (bind _returnvalue_2 (`GameplayStatics.SaveGameToSlot` (`self.SaveGameClass`) (`self.SaveSlot`)))
    (`|ExecutionSequence`
      (:`then_0`
        (`KismetSystemLibrary.PrintString` (`KismetStringLibrary.Concat_StrStr` "Save: " (`KismetStringLibrary.Conv_BoolToString` _returnvalue_2)) (`self.ShowPrint`)))
      (:`then_1`
        (return _returnvalue_2)))))

(fn `UserConstructionScript`)